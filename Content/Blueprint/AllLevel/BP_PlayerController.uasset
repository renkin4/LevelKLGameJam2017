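; Player controller for a hero-and-mission game, handling headquarters UI startup and mission success odds.
; On BeginPlay it initializes the headquarters through BP_Hud, then switches to UI-only input on that widget with the mouse cursor shown.
; CalculateSuccessRate compares selected heroes' class-default traits to the selected mission's, removing matched mission traits as it goes.
; The success rate is the match count divided by twice the mission's trait count.
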(event EventBeginPlay
  (Utilities|FlowControl|Sequence
    (:then_0
      ;[1 1 1] TODo Set GameMode
      (Class|WidgetBlueprintLibrary|SetFocustoGameViewport)
      (bind _asbp_hud (Utilities|Casting|CastToBP_Hud (HUD|GetHUD)))
      (Variables|Default|SetHUDRef _asbp_hud)
      (bind _widgetref (Default|InitializeHeadquarter (Variables|Default|GetHUDRef)))
      (Input|SetInputModeUIOnly self _widgetref "LockAlways")
      (Variables|Default|SetbShowMouseCursor true))))

(fn ConstructionScript)

(fn CalculateSuccessRate
  (bind _currentselectedmission (Variables|Default|GetCurrentSelectedMission))
  (bind _currentselectedheroes (Variables|Default|GetCurrentSelectedHeroes))
  (bind _missionrequirement (Utilities|GetClassDefaults _currentselectedmission))
  (bind _missiontraits (Utilities|Struct|BreakMissionRequirement _missionrequirement))
  (if (Utilities|Array|IsValidIndex _currentselectedheroes)
    (LocalVariables|SetMissionTraits _missiontraits)
    (for _array_element _currentselectedheroes
      (for _array_element_2 (.HeroesTraits (Utilities|Struct|BreakHeroesStats (Utilities|GetClassDefaults _array_element)))
        (for (_array_element_3 _array_index) (LocalVariables|GetMissionTraits)
          (if (Utilities|Enum|Equal(Enum) _array_element_2 _array_element_3)
            (LocalVariables|SetSimilar (+ (LocalVariables|GetSimilar) 1))
            (Utilities|Array|Add (LocalVariables|GetIndexToDelete) _array_index)))
        (for _array_element_4 (LocalVariables|GetIndexToDelete)
          (Utilities|Array|RemoveIndex (LocalVariables|GetMissionTraits) _array_element_4))
        (Utilities|Array|Clear (LocalVariables|GetIndexToDelete))))
    (Variables|Default|SetSuccessRate (/ (Math|Conversions|ToFloat(Integer) (LocalVariables|GetSimilar)) (* (Utilities|Array|Length _missiontraits) 2.0)))
    (return (/ (Math|Conversions|ToFloat(Integer) (LocalVariables|GetSimilar)) (* (Utilities|Array|Length _missiontraits) 2.0)))))